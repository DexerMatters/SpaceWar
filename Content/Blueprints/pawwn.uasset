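; Player pawn for a free-flight shooter: a cube that flies constantly along its facing and fires Bullets on left click.
; Tick steers from accumulated mouse offset to screen center; W adds speed, S pauses flight.
; Holding B ramps a time-limited boost with widening FOV, re-enabled after FOV eases back.
; Die enables physics and shows Diewindow, but its call after swept movement is disabled by a constant-false condition.
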(event `self.ReceiveBeginPlay`)

(event `restart`
  (bind _cube (`self.Cube`))
  (`self.K2_SetActorLocation` (`KismetMathLibrary.MakeVector` (.x (`self.K2_GetActorLocation`)) (+ (.y (`self.K2_GetActorLocation`)) 100.0) (.z (`self.K2_GetActorLocation`))) true)
  (`PrimitiveComponent.SetSimulatePhysics` _cube false)
  (`PrimitiveComponent.SetEnableGravity` _cube false))

(event `self.ReceiveTick`
  (params (DeltaSeconds :type "Float (single-precision)"))
  (bind _focus (`self.focus`))
  (bind `_灵敏度` (`self.灵敏度`))
  (bind _camera (`self.Camera`))
  (bind _focus_2 (`self.focus`))
  (bind _time (`self.time`))
  (bind (_x _y) (`KismetMathLibrary.BreakVector2D` (`WidgetLayoutLibrary.GetViewportSize`)))
  (bind (_locationx _locationy) (`PlayerController.GetMousePosition` (`GameplayStatics.GetPlayerController` 0)))
  (`|ExecutionSequence`
    (:`then_0`
      (if (`self.enableAntoView`)
        ;[1 1 1] 视角
        (`SceneComponent.K2_SetWorldRotation` (`self.Cube`) (`KismetMathLibrary.MakeRotator` 0.0 (* (stale _output_get_2) `_灵敏度`) (- 0.0 (* `_灵敏度` (stale _output_get)))) false true)))
    (:`then_1`
      (`|ExecutionSequence`
        (:`then_0`
          (bind _output_get (set `self.moveX` (+ (`self.moveX`) (- (/ _x 2.0) _locationx)))))
        (:`then_1`
          (bind _output_get_2 (set `self.moveY` (+ (`self.moveY`) (- (/ _y 2.0) _locationy)))))))
    (:`then_2`
      ;[1 1 1] 加速系统
      (if (`self.isTouchedPower`)
        (`|ExecutionSequence`
          (:`then_0`
            (set `self.time` (+ _time 1))
            (bind _output_get_3 (set `self.focus` (+ _focus 0.5)))
            (if (> (`self.focus`) 169.0)
              (`CameraComponent.SetFieldOfView` _camera 169.0)
              (else
                (`CameraComponent.SetFieldOfView` _camera _output_get_3))))
          (:`then_1`
            (if (`self.enableAntoFlying`)
              (`self.Move with speed` (* (`self.time`) 6.0)))))
        (else
          (set `self.time` 0)
          (if (`KismetMathLibrary.NearlyEqual_FloatFloat` _focus 90.0 0.1)
            (bind _output_get_4 (set `self.focus` 90.0))
            (`CameraComponent.SetFieldOfView` _camera _output_get_4)
            (set `self.enableTouch` true)
            (else
              (set `self.enableTouch` false)
              (bind _output_get_5 (set `self.focus` (- _focus_2 (/ (- _focus_2 90.0) 10.0))))
              (`CameraComponent.SetFieldOfView` _camera _output_get_5))))))
    (:`then_3`
      (if (== _time 135)
        (set `self.isTouchedPower` false)))
    (:`then_4`
      (if (`self.enableAntoFlying`)
        ;[1 1 1] 移动
        (if (`self.isTouchedForward`)
          (`self.Move with speed` (`self.speed_2`)))))
    (:`then_5`
      (if (`self.enableAntoFlying`)
        (`self.Move with speed` 12.0)))))

(event `Key|B`
  (params (Key :type "Key Structure"))
  ;[1 1 1] 按键
  (:`Pressed`
    (if (`self.enableTouch`)
      (set `self.isTouchedPower` true)))
  (:`Released`
    (if (`self.enableTouch`)
      (set `self.isTouchedPower` false))))

(event `Key|W`
  (params (Key :type "Key Structure"))
  ;[1 1 1] 按键
  (:`Pressed`
    (set `self.isTouchedForward` true))
  (:`Released`
    (set `self.isTouchedForward` false)))

(event `Key|S`
  (params (Key :type "Key Structure"))
  ;[1 1 1] 按键
  (:`Pressed`
    (set `self.enableAntoFlying` false))
  (:`Released`
    (set `self.enableAntoFlying` true)))

(event `Key|LeftMouseButton`
  (params (Key :type "Key Structure"))
  ;[1 1 1] 按键
  (:`Pressed`
    (`|SpawnActorFromClass` "/Game/Blueprints/bullet.bullet_C" (`KismetMathLibrary.MakeTransform` (`SceneComponent.K2_GetComponentLocation` (`self.Cube`)) (`SceneComponent.K2_GetComponentRotation` (`self.Cube`))) "Undefined" "OverrideRootScale" null null)))

(fn `die`
  (bind _cube (`self.Cube`))
  (set `self.enableAntoFlying` false)
  (set `self.enableAntoView` false)
  (`|ExecutionSequence`
    (:`then_0`
      (`PrimitiveComponent.SetEnableGravity` _cube true))
    (:`then_1`
      (`PrimitiveComponent.SetSimulatePhysics` _cube true))
    (:`then_2`
      (bind _returnvalue (`|CreateWidget` "/Game/Blueprints/diewindow.diewindow_C"))
      (`UserWidget.AddToViewport` _returnvalue 0)
      (set `PlayerController.bShowMouseCursor` true (`GameplayStatics.GetPlayerController` 0)))))

(fn `Move with speed`
  (params (NewParam :type "Float (double-precision)"))
  (bind _cube (`self.Cube`))
  (bind _sweephitresult (`SceneComponent.K2_SetWorldLocation` _cube (+ (`SceneComponent.K2_GetComponentLocation` _cube) (* (`KismetMathLibrary.Conv_RotatorToVector` (`SceneComponent.K2_GetComponentRotation` _cube)) NewParam)) true true))
  (if (and false false)
    (`self.die`)))

(fn `UserConstructionScript`)