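; Bullet projectile actor that flies along its facing direction and removes itself after a short lifetime.
; On BeginPlay it sets the linear velocity of its physics-driven Cube mesh to the actor's forward vector times Speed.
; Tick increments a Life counter and destroys the actor at a fixed count, so lifetime depends on frame rate.
; It has no hit or overlap logic.
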(event `self.ReceiveBeginPlay`
  (`PrimitiveComponent.SetPhysicsLinearVelocity` (`self.Cube`) (* (`KismetMathLibrary.Conv_RotatorToVector` (`self.K2_GetActorRotation`)) (`self.speed`)) false "None")
  (`PrimitiveComponent.SetPhysicsLinearVelocity` (`self.StaticMesh`) (* (`KismetMathLibrary.Conv_RotatorToVector` (`self.K2_GetActorRotation`)) (`self.speed`)) false "None"))

(event `self.ReceiveTick`
  (params (DeltaSeconds :type "Float (single-precision)"))
  (bind _life (`self.life`))
  (`/Engine/EditorBlueprintResources/StandardMacros.IncrementInt` _life
    (:`  `
      (if (== _life 200)
        (`self.K2_DestroyActor`)))))

(fn `UserConstructionScript`)