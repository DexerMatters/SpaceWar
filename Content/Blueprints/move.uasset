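; Blueprint function that is meant to shift an actor along world X, Y or Z by a length, chosen by an integer mode.
; The entry connects to nothing, so neither the variable assignments nor the move sequence runs.
; The unwired logic uses SetActorLocation without sweep, but its Z branch adds the length to the X coordinate.
; The actor variable's setter assigns None instead of the input.
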(fn `move`
  (params (Actor :type "Actor Object Reference") (Length :type "Float (double-precision)") (Mode :type Integer))
  (locals (Actorr :type "AbstractNavData Object Reference") (Lengthh :type "Float (double-precision)") (Modee :type Integer)))